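; TestPawn is a test pawn in XBall for trying out area damage on blocks with a mouse click.
; Left click runs a debug-drawn object line trace from the pawn along the control rotation.
; It calls HitBlockAtRange just past the trace's hit location and draws a debug sphere showing the range.
; Pitch input, movement input and a smaller debug sphere are left unconnected.
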(event `Key|LeftMouseButton`
  (params (Key :type "Key Structure"))
  (bind _returnvalue (`self.K2_GetActorLocation`))
  (bind _returnvalue_2 (`KismetMathLibrary.GetForwardVector` (`self.GetControlRotation`)))
  (:`Pressed`
    (bind _outhit (`KismetSystemLibrary.LineTraceSingleForObjects` :`Start` _returnvalue :`End` (+ _returnvalue (* _returnvalue_2 10000)) :`ObjectTypes` (`|MakeArray` "ObjectTypeQuery1" "ObjectTypeQuery2" "ObjectTypeQuery4" "ObjectTypeQuery5" "ObjectTypeQuery6" :!type "EObjectTypeQuery Enum") :`bTraceComplex` true :`DrawDebugType` "ForDuration"))
    (bind _returnvalue_3 (+ (`.Location` (`GameplayStatics.BreakHitResult` _outhit)) _returnvalue_2))
    (`MyBPFuncLib.HitBlockAtRange` _returnvalue_3 (1000.0 1000.0 1000.0) 70.0)
    (`KismetSystemLibrary.DrawDebugSphere` _returnvalue_3 1000.0 12 (struct :`R` 1.0 :`G` 1.0 :`B` 1.0 :`A` 1.0) 10.0)))

(fn `UserConstructionScript`)