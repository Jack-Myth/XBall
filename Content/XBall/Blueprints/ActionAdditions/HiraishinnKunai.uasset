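; HiraishinnKunai is a thrown kunai actor tied to a Skill, damaging actors it overlaps.
; On the authority, a delayed loop steps it forward with swept offsets until a blocking hit or the loop's end, then sets its box to block all channels.
; It has Health and can be damaged; at zero it starts the Skill's cooldown and destroys itself.
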(event `ReGenCol`
  (`PrimitiveComponent.SetCollisionResponseToAllChannels` (`self.Box`) "ECR_Block"))

(event `self.ReceiveBeginPlay`
  (`/Engine/EditorBlueprintResources/ActorMacros.Switch Has Authority`
    (:`Authority`
      (`/Game/MacroLibrary.ForLoopWithDelay` 0 1000 0.02 :!label _label
        (:`LoopBody`
          (bind _sweephitresult (`self.K2_AddActorWorldOffset` (* (`self.GetActorForwardVector`) 30) true))
          (if (`GameplayStatics.BreakHitResult` _sweephitresult)
            (goto _label :!via `Break`)))
        (:`Complited`
          (`self.ReGenCol` :!label _label_2))
        (:`Breaked`
          (goto _label_2))))))

(event `self.ReceiveAnyDamage`
  (params (Damage :type "Float (single-precision)") (DamageType :type "DamageType Object Reference") (InstigatedBy :type "Controller Object Reference") (DamageCauser :type "Actor Object Reference"))
  (bind _output_get (set `self.Health` (- (`self.Health`) Damage)))
  (if (<= _output_get 0.0)
    (`/Game/XBall/Blueprints/Actions/Skills/Hiraishinn.BeginCoolDown` (`self.Skill`))
    (`self.K2_DestroyActor`)))

(event `self.ReceiveActorBeginOverlap`
  (params (OtherActor :type "Actor Object Reference"))
  (`GameplayStatics.ApplyDamage` OtherActor 30.0 (`self.GetInstigatorController`) self))

(fn `UserConstructionScript`)