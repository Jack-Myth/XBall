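; Proximity mine that blinks and beeps, then explodes with radial damage, block damage in range, and effects.
; A looping timer runs ChangeMineLight to toggle the material glow and point light.
; On the authority, an XBallBase overlap from a controller other than the instigator speeds up the blink and detonates after one second.
; Any damage detonates it immediately through the same explosion path, guarded by IsBoomed.
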(event `ReadyBoom`
  (`KismetSystemLibrary.K2_SetTimer` null "ChangeMineLight" 0.05 true))

(event `SpawnEmitter`
  (bind _returnvalue (`self.K2_GetActorLocation`))
  (`GameplayStatics.SpawnEmitterAtLocation` "/Game/HDParticlePack/Particles/P_ClusterMini.P_ClusterMini" _returnvalue (struct) (3.0 3.0 3.0))
  (`GameplayStatics.PlaySoundAtLocation` "/Game/XBall/Sounds/MineBoom.MineBoom" _returnvalue (struct) 1.0 1.0 0.0 "/Game/XBall/Blueprints/DefSoundAttenuation.DefSoundAttenuation")
  (`GameplayStatics.PlayWorldCameraShake` "/Game/XBall/Blueprints/DefCameraShake.DefCameraShake_C" (`self.K2_GetActorLocation`) 500.0 1000.0))

(event `self.ReceiveBeginPlay`
  (`KismetSystemLibrary.K2_SetTimer` null "ChangeMineLight" 0.5 true)
  (bind _returnvalue (`PrimitiveComponent.CreateDynamicMaterialInstance` (`self.Sphere`) 0 null))
  (set `self.MineDMI` _returnvalue))

(event `self.ReceiveAnyDamage`
  (params (Damage :type "Float (single-precision)") (DamageType :type "DamageType Object Reference") (InstigatedBy :type "Controller Object Reference") (DamageCauser :type "Actor Object Reference"))
  (bind _returnvalue (`self.K2_GetActorLocation`))
  (if (not (`self.IsBoomed`))
    (set `self.IsBoomed` true :!label _label)
    (`self.SpawnEmitter`)
    (`GameplayStatics.ApplyRadialDamageWithFalloff` :`BaseDamage` 150.0 :`Origin` _returnvalue :`DamageInnerRadius` 10.0 :`DamageOuterRadius` 500.0 :`DamageFalloff` 1.5 :`DamageTypeClass` "/Game/XBall/Blueprints/DamageAll.DamageAll_C" :`DamageCauser` self :`InstigatedByController` (`self.GetInstigatorController`) :`DamagePreventionChannel` "ECC_WorldStatic")
    (`MyBPFuncLib.HitBlockAtRange` _returnvalue (300.0 300.0 300.0) 200.0)
    (`self.K2_DestroyActor`)))

(event `self.Sphere1.OnComponentBeginOverlap`
  (params (OverlappedComponent :type "PrimitiveComponent Object Reference") (OtherActor :type "Actor Object Reference") (OtherComp :type "PrimitiveComponent Object Reference") (OtherBodyIndex :type Integer) (bFromSweep :type Boolean) (SweepResult :type "HitResult Structure (by ref)"))
  (`/Engine/EditorBlueprintResources/ActorMacros.Switch Has Authority`
    (:`Authority`
      (bind _asxball_base (cast `XBallBase` OtherActor))
      (if (!= (`Pawn.GetController` _asxball_base) (`self.GetInstigatorController`))
        (`self.ReadyBoom`)
        (`KismetSystemLibrary.Delay` 1.0)
        (goto _label)))))

(fn `ChangeMineLight`
  (bind _minedmi (`self.MineDMI`))
  (bind _pointlight (`self.PointLight`))
  (bind _output_get (set `self.IsMineRed` (not (`self.IsMineRed`))))
  (if _output_get
    (`MaterialInstanceDynamic.SetScalarParameterValue` _minedmi "SelfColorLight" 1.0)
    (`SceneComponent.SetVisibility` _pointlight true false)
    (`GameplayStatics.PlaySoundAtLocation` "/Game/XBall/Sounds/dididi.dididi" (`self.K2_GetActorLocation`) (struct) 1.0 1.0 0.0 "/Game/XBall/Blueprints/MineSA.MineSA")
    (else
      (`MaterialInstanceDynamic.SetScalarParameterValue` _minedmi "SelfColorLight" 0.0)
      (`SceneComponent.SetVisibility` _pointlight false false))))

(fn `UserConstructionScript`)