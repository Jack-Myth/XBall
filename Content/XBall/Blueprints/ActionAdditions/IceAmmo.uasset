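; IceAmmo is an ice projectile actor that damages what it hits and temporarily slows struck characters.
; On BeginPlay, the authority moves it forward in swept steps through a delayed loop instead of a movement component, destroying it if the loop finishes.
; A blocking hit hides the sphere, spawns an impact emitter and applies radial damage.
; A directly hit character's walk speed drops for five seconds, then returns to a fixed value.
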(event `HideAndEmitter`
  (params (Location :type "Vector Structure") (Rotation :type "Rotator Structure"))
  (`SceneComponent.SetVisibility` (`self.Sphere`) false true)
  (`GameplayStatics.SpawnEmitterAtLocation` "/Game/InfinityBladeEffects/Effects/FX_Monsters/FX_Monster_FrostGiant/ICE/P_ArmBuildUp01.P_ArmBuildUp01" Location Rotation)
  (`PrimitiveComponent.SetCollisionEnabled` (`self.Sphere`) "NoCollision"))

(event `IncreaseSpeed`
  (params (Target :type "Character Object Reference"))
  (set `CharacterMovementComponent.MaxWalkSpeed` 600.0 (`Character.CharacterMovement` Target)))

(event `DecreaseSpeed`
  (params (Target :type "Character Object Reference"))
  (set `CharacterMovementComponent.MaxWalkSpeed` 100.0 (`Character.CharacterMovement` Target)))

(event `self.ReceiveBeginPlay`
  (`/Engine/EditorBlueprintResources/ActorMacros.Switch Has Authority`
    (:`Authority`
      (`/Game/MacroLibrary.ForLoopWithDelay` 0 1000 0.02 :!label _label
        (:`LoopBody`
          (bind _sweephitresult (`self.K2_AddActorWorldOffset` (* (`self.GetActorForwardVector`) 20) true))
          (bind (_bblockinghit _binitialoverlap _time _distance _location _impactpoint _normal _impactnormal _physmat _hitactor) (`GameplayStatics.BreakHitResult` _sweephitresult))
          (if _bblockinghit
            (`|ExecutionSequence`
              (:`then_0`
                (goto _label :!via `Break`))
              (:`then_1`
                (bind (_returnvalue_roll _returnvalue_pitch _returnvalue_yaw) (`KismetMathLibrary.BreakRotator` (`KismetMathLibrary.FindLookAtRotation` (`KismetMathLibrary.MakeVector` 0.0) _impactnormal)))
                (`self.HideAndEmitter` _impactpoint (`KismetMathLibrary.MakeRotator` _returnvalue_roll (+ _returnvalue_pitch 90.0) _returnvalue_yaw))
                (`GameplayStatics.ApplyRadialDamage` :`BaseDamage` 50.0 :`Origin` _impactpoint :`DamageRadius` 200.0 :`DamageCauser` self :`InstigatedByController` (`self.GetInstigatorController`) :`DamagePreventionChannel` "ECC_WorldStatic")
                (`/Engine/EditorBlueprintResources/StandardMacros.IsValid` _hitactor
                  (:`Is Valid`
                    (bind _ascharacter (cast `Character` _hitactor)
                      (:`then`
                        (`self.DecreaseSpeed` _ascharacter)
                        (`KismetSystemLibrary.Delay` 5.0)
                        (`self.IncreaseSpeed` _ascharacter))
                      (:`CastFailed`
                        _)))
                  (:`Is Not Valid`
                    _))
                (`self.K2_DestroyActor`)))))
        (:`Complited`
          (`self.K2_DestroyActor`))))))

(fn `UserConstructionScript`)