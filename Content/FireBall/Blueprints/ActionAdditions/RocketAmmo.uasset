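; Rocket projectile that explodes on impact, damaging nearby blocks and applying radial damage around the hit point.
; On BeginPlay it copies its Velocity variable into ProjectileMovement and activates it.
; Hits are handled only on authority and ignore the instigator, running block damage, explosion emitter and radial damage before the actor destroys itself.
; Block damage reaches farther and has a higher maximum than the radial damage, which is credited to the DamageBy controller.
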(event `SpawnEmitter`
  (params (Location :type "Vector Structure"))
  (`GameplayStatics.SpawnEmitterAtLocation` "/Game/InfinityBladeEffects/Effects/FX_Monsters/FX_Monster_Gruntling/Bomber/P_BomberExplode.P_BomberExplode" Location (`self.K2_GetActorRotation`)))

(event `self.ReceiveBeginPlay`
  (bind _projectilemovement (`self.ProjectileMovement`))
  (set `MovementComponent.Velocity` (`self.Velocity`) _projectilemovement)
  (`ActorComponent.Activate` _projectilemovement true))

(event `self.ReceiveHit`
  (params (MyComp :type "PrimitiveComponent Object Reference") (Other :type "Actor Object Reference") (OtherComp :type "PrimitiveComponent Object Reference") (bSelfMoved :type Boolean) (HitLocation :type "Vector Structure") (HitNormal :type "Vector Structure") (NormalImpulse :type "Vector Structure") (Hit :type "HitResult Structure (by ref)"))
  (`/Engine/EditorBlueprintResources/ActorMacros.Switch Has Authority`
    (:`Authority`
      (if (not (== Other (`self.Instigator`)))
        (`MyBPFuncLib.HitBlockAtRange` HitLocation (500.0 500.0 500.0) 300.0)
        (`self.SpawnEmitter` HitLocation)
        (`GameplayStatics.ApplyRadialDamage` :`BaseDamage` 90.0 :`Origin` HitLocation :`DamageRadius` 200.0 :`DamageCauser` (`self.Instigator`) :`InstigatedByController` (`self.DamageBy`))
        (`self.K2_DestroyActor`)))))

(fn `UserConstructionScript`)