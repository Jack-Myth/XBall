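; Machine gun projectile actor that flies forward, damaging the actor and block it hits.
; On BeginPlay the authority drives movement with a timed delay loop of swept forward offsets instead of a movement component.
; A blocking hit applies damage, draws a debug sphere, spawns an impact particle through the SpawnEmitter event and destroys the actor.
; The actor also destroys itself when the loop completes without a hit.
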(event `SpawnEmitter`
  (params (Location :type "Vector Structure"))
  (`GameplayStatics.SpawnEmitterAtLocation` "/Game/InfinityBladeEffects/Effects/FX_Monsters/FX_Monster_Gruntling/Notifies/P_Death_PickImpact.P_Death_PickImpact" Location (`self.K2_GetActorRotation`)))

(event `self.ReceiveBeginPlay`
  (`/Engine/EditorBlueprintResources/ActorMacros.Switch Has Authority`
    (:`Authority`
      (`/Game/MacroLibrary.ForLoopWithDelay` 0 1000 0.02 :!label _label
        (:`LoopBody`
          (bind _sweephitresult (`self.K2_AddActorWorldOffset` (* (`self.GetActorForwardVector`) 100) true))
          (bind (_bblockinghit _binitialoverlap _time _distance _location _impactpoint _normal _impactnormal _physmat _hitactor) (`GameplayStatics.BreakHitResult` _sweephitresult))
          (if _bblockinghit
            (`GameplayStatics.ApplyDamage` _hitactor 30.0)
            (`KismetSystemLibrary.DrawDebugSphere` _impactpoint 5.0 12 (struct :`R` 1.0 :`G` 1.0 :`B` 1.0 :`A` 1.0) 100.0)
            (`MyBPFuncLib.HitBlockAtLocationWithNormal` _impactpoint _impactnormal 80.0)
            (`self.SpawnEmitter` _impactpoint)
            (`self.K2_DestroyActor`)
            (goto _label :!via `Break`)))
        (:`Complited`
          (`self.K2_DestroyActor`))))))

(fn `UserConstructionScript`)